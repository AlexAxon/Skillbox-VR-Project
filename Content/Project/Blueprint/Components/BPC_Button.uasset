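; VR push-button component that BP_VRPawn's hand grab collisions physically press, in either momentary or toggle mode.
; On overlap it enables tick and follows the hand along local Z, clamped to a maximum travel.
; When released it interpolates back toward its starting position and can switch tick off.
; Depth past a threshold drives the state, with a minimum time between changes, firing ButtonPressed and swapping green/red materials.
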(event `self.ReceiveBeginPlay`
  (add `self.OnComponentBeginOverlap` (`|CreateDelegate` :!event `ComponentBeginOverlap`))
  (add `self.OnComponentEndOverlap` (`|CreateDelegate` :!event `ComponentEndOverlap`))
  (set `self.StartupTransform` (`self.GetRelativeTransform`)))

(event `ComponentBeginOverlap` :!signature `self.OnComponentBeginOverlap`
  (params (OverlappedComponent :type "PrimitiveComponent Object Reference") (OtherActor :type "Actor Object Reference") (OtherComp :type "PrimitiveComponent Object Reference") (OtherBodyIndex :type Integer) (bFromSweep :type Boolean) (SweepResult :type "HitResult Structure (by ref)"))
  (bind _asbp_vrpawn (cast `/Game/Project/Blueprint/Game/BP_VRPawn` OtherActor))
  (bind _output_get (set `self.FocusActor` _asbp_vrpawn))
  (bind _leftgrapcollision (`/Game/Project/Blueprint/Game/BP_VRPawn.LeftGrapCollision` _output_get))
  (bind _rightgrapcollision (`/Game/Project/Blueprint/Game/BP_VRPawn.RightGrapCollision` _output_get))
  (bind _returnvalue (== OtherComp _rightgrapcollision))
  (if (or (== _leftgrapcollision OtherComp) _returnvalue)
    (bind _output_get_2 (set `self.FocusedComponent` (select `bool` _returnvalue :`false` _leftgrapcollision :`true` _rightgrapcollision)))
    (`self.StartButtonTransforming` _output_get_2)))

(event `ComponentEndOverlap` :!signature `self.OnComponentEndOverlap`
  (params (OverlappedComponent :type "PrimitiveComponent Object Reference") (OtherActor :type "Actor Object Reference") (OtherComp :type "PrimitiveComponent Object Reference") (OtherBodyIndex :type Integer))
  (if (`self.bIsEnebled`)
    (if (== OtherActor (`self.FocusActor`))
      (set `self.FocusActor` null)
      (set `self.FocusedComponent` null)
      (set `self.bIsEnebled` false))))

(event `self.ReceiveTick`
  (params (DeltaSeconds :type "Float (single-precision)"))
  (`|ExecutionSequence`
    (:`then_0`
      (if (`self.bIsEnebled`)
        (`self.UpdateButtonLocation`)
        (elif (not (`self.bLerping`))
          (set `self.FocusActor` null)
          (set `self.FocusedComponent` null)
          (set `self.bLerping` true))))
    (:`then_1`
      (`self.LerpReturnMovingButton`)
      (`self.UpdateButtonStateAndColor`))))

(fn `CheckButtonPressed`
  (params (State :type Boolean))
  (returns (Success :type Boolean))
  (bind _btogglethistouch (`self.bToggleThisTouch`))
  (if (>= (`KismetMathLibrary.GetTotalSeconds` (- (`KismetMathLibrary.Now`) (`self.LastToggleTime`))) (`self.MaxTimeBetweenToggle`))
    (if (`self.bTogglingButton`)
      (if _btogglethistouch
        (set `self.bToggleThisTouch` (not _btogglethistouch))
        (bind _output_get (set `self.bButtonState` (not (`self.bButtonState`))))
        (`self.ButtonPressed` _output_get)
        (set `self.LastToggleTime` (`KismetMathLibrary.Now`))
        (return _output_get)
        (else
          (set `self.bToggleThisTouch` (not (`self.bToggleThisTouch`)))))
      (else
        (bind _output_get_2 (set `self.bButtonState` (`local.State`)))
        (`self.ButtonPressed` _output_get_2)
        (set `self.LastToggleTime` (`KismetMathLibrary.Now`))
        (return (`self.bButtonState`))))
    (else
      (return false))))

(fn `GetCurrentTransform`
  (returns (CurrentTransform :type "Transform Structure"))
  (`self.FocusActor`
    (:`then`
      (return (`KismetMathLibrary.ComposeTransforms` (`self.StartupTransform`) (`self.K2_GetComponentToWorld` (`self.GetAttachParent`)))))
    (:`else`
      (return (`self.StartupTransform`)))))

(fn `LerpReturnMovingButton`
  (bind _startuptransform_location (`KismetMathLibrary.BreakTransform` (`self.StartupTransform`)))
  (bind _returnvalue (`KismetMathLibrary.VInterpTo_Constant` (`self.RelativeLocation`) _startuptransform_location (`GameplayStatics.GetWorldDeltaSeconds`) (`self.ReturnSpeed`)))
  (if (`self.bLerping`)
    (`self.K2_SetRelativeLocation` _returnvalue)
    (if (== _returnvalue (0.0 0.0 0.0) :`ErrorTolerance` 0.0001)
      (set `self.bLerping` false)
      (`self.SetComponentTickEnabled` false))))

(fn `SetButtonColor`
  (params (State :type Boolean))
  (if State
    (`self.SetMaterial` 0 "/Game/Project/Materials/M_ColorGreen.M_ColorGreen")
    (else
      (`self.SetMaterial` 0 "/Game/Project/Materials/M_ColorRed.M_ColorRed"))))

(fn `StartButtonTransforming`
  (params (Component :type "SphereComponent Object Reference"))
  (bind _currenttransform (`self.GetCurrentTransform`))
  (bind (_returnvalue_x _returnvalue_y _returnvalue_z) (`KismetMathLibrary.BreakVector` (`KismetMathLibrary.InverseTransformLocation` _currenttransform (`self.K2_GetComponentLocation`))))
  (bind (_returnvalue_x_2 _returnvalue_y_2 _returnvalue_z_2) (`KismetMathLibrary.BreakVector` (`KismetMathLibrary.InverseTransformLocation` _currenttransform (`self.K2_GetComponentLocation` Component))))
  (set `self.StartupLocalZ` _returnvalue_z_2)
  (set `self.StartupComponentZ` _returnvalue_z)
  (`self.SetComponentTickEnabled` true)
  (set `self.bLerping` false)
  (set `self.bToggleThisTouch` true)
  (set `self.bIsEnebled` true))

(fn `UpdateButtonLocation`
  (bind (_returnvalue_x _returnvalue_y _returnvalue_z) (`KismetMathLibrary.BreakVector` (`KismetMathLibrary.InverseTransformLocation` (`self.GetCurrentTransform`) (`self.K2_GetComponentLocation` (`self.FocusedComponent`)))))
  (bind _returnvalue (`KismetMathLibrary.FClamp` (- (`self.StartupLocalZ`) _returnvalue_z) 0.0 (`self.MaxMoveDistance`)))
  (if (> _returnvalue 0.0)
    (`self.K2_SetRelativeLocation` (`KismetMathLibrary.TransformLocation` (`self.StartupTransform`) (`KismetMathLibrary.MakeVector` 0.0 0.0 (`KismetMathLibrary.FClamp` (+ (`self.StartupComponentZ`) (* _returnvalue -1.0)) (* (`self.MaxMoveDistance`) -1.0)))))))

(fn `UpdateButtonStateAndColor`
  (bind (_returnvalue_x _returnvalue_y _returnvalue_z) (`KismetMathLibrary.BreakVector` (`KismetMathLibrary.InverseTransformLocation` (`self.StartupTransform`) (`self.RelativeLocation`))))
  (bind _returnvalue (<= _returnvalue_z (+ (* (`self.TogglingZoneHeight`) -1.0) 0.001)))
  (if (!= _returnvalue (`self.bButtonState`))
    (`/Engine/EditorBlueprintResources/StandardMacros.DoOnce` false :!label _label
      (:`Completed`
        (if (`self.bTogglingButton`)
          (if (`self.bToggleThisTouch`)
            (bind _success (`self.CheckButtonPressed` (`self.bButtonState`)))
            (`self.SetButtonColor` _success))
          (else
            (bind _output_get (set `self.bButtonState` _returnvalue))
            (`self.CheckButtonPressed` _output_get)
            (`self.SetButtonColor` _output_get)))))
    (else
      (goto _label :!via `Reset`))))