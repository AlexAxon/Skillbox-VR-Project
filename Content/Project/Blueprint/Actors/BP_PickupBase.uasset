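; BP_PickupBase is a base pickup actor whose grippable mesh can be gripped and dropped, with its static mesh set in construction.
; On grip it disables physics and attaches to the gripping component, snapping with offsets from a "Grip" socket if present, otherwise keeping its world pose.
; On drop it re-enables physics and detaches.
; GetStatus always returns the same enum value.
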(event `self.ReceiveBeginPlay`
  (add `/Game/Project/Blueprint/Components/BPC_GripableMesh.OnGrip` (`self.BPC_GripableMesh`) (`|CreateDelegate` :!event `OnGrip`))
  (add `/Game/Project/Blueprint/Components/BPC_GripableMesh.OnDrop` (`self.BPC_GripableMesh`) (`|CreateDelegate` :!event `OnDrop`)))

(event `OnGrip`
  (params (`Parent Component` :type "SphereComponent Object Reference"))
  (bind _returnvalue (`SceneComponent.GetSocketTransform` (`self.BPC_GripableMesh`) "Grip" "RTS_Actor"))
  (`PrimitiveComponent.SetSimulatePhysics` (`self.BPC_GripableMesh`) false)
  (if (`SceneComponent.DoesSocketExist` (`self.BPC_GripableMesh`) "Grip")
    (`SceneComponent.K2_AttachToComponent` (`self.BPC_GripableMesh`) `Parent Component` "None" "SnapToTarget" "SnapToTarget" "KeepRelative" true)
    (`SceneComponent.K2_AddRelativeLocation` (`self.BPC_GripableMesh`) (* (`SceneComponent.K2_GetComponentScale` (`self.BPC_GripableMesh`)) (.location (`KismetMathLibrary.InvertTransform` _returnvalue))) false false)
    (`SceneComponent.K2_AddLocalRotation` (`self.BPC_GripableMesh`) (.rotation _returnvalue) false false)
    (else
      (`SceneComponent.K2_AttachToComponent` (`self.BPC_GripableMesh`) `Parent Component` "None" "KeepWorld" "KeepWorld" "KeepRelative" true))))

(event `OnDrop`
  (`PrimitiveComponent.SetSimulatePhysics` (`self.BPC_GripableMesh`) true)
  (`SceneComponent.K2_DetachFromComponent` (`self.BPC_GripableMesh`) "KeepRelative" "KeepRelative" "KeepRelative" true))

(fn `GetStatus`
  (returns (GripBy :type "/Game/Project/Blueprint/Data/Enum_HandType Enum"))
  (return "NewEnumerator0"))

(fn `UserConstructionScript`
  (`StaticMeshComponent.SetStaticMesh` (`self.BPC_GripableMesh`) (`self.Mesh`)))