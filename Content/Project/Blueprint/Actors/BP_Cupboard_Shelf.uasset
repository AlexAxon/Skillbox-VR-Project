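; BP_Cupboard_Shelf is a cupboard shelf actor that slides out and back when its handle is gripped.
; The handle's grip and drop events set or clear the interactor component, while hover events switch its material between green and gray.
; While gripped, Tick converts the interactor position to actor space, offsets it by the handle position, and moves Axis along local X, clamped to MaxDistance.
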(event `self.ReceiveBeginPlay`
  (add `/Game/Project/Blueprint/Components/BPC_GripableMesh.OnGrip` (`self.SlelfHandle`) (`|CreateDelegate` :!event `EventOnGrip`))
  (add `/Game/Project/Blueprint/Components/BPC_GripableMesh.OnDrop` (`self.SlelfHandle`) (`|CreateDelegate` :!event `EventOnDrop`))
  (add `/Game/Project/Blueprint/Components/BPC_GripableMesh.OnHover` (`self.SlelfHandle`) (`|CreateDelegate` :!event `EventOnHover`))
  (add `/Game/Project/Blueprint/Components/BPC_GripableMesh.OnUnhover` (`self.SlelfHandle`) (`|CreateDelegate` :!event `EventOnUnhover`)))

(event `self.ReceiveTick`
  (params (DeltaSeconds :type "Float (single-precision)"))
  (`self.Interactor`
    (:`then`
      (`SceneComponent.K2_SetRelativeLocation` (`self.Axis`) (`KismetMathLibrary.MakeVector` (`KismetMathLibrary.FClamp` (`self.CalculateLocation`) 0.0 (`self.MaxDistance`))) false false))
    (:`else`)))

(event `EventOnGrip`
  (params (`Parent Component` :type "SphereComponent Object Reference"))
  (set `self.Interactor` `Parent Component`))

(event `EventOnDrop`
  (set `self.Interactor` null))

(event `EventOnHover`
  (`PrimitiveComponent.SetMaterial` (`self.SlelfHandle`) 0 "/Game/Project/Materials/M_ColorGreen.M_ColorGreen"))

(event `EventOnUnhover`
  (`PrimitiveComponent.SetMaterial` (`self.SlelfHandle`) 0 "/Game/Project/Materials/M_ColorGray.M_ColorGray"))

(fn `CalculateLocation`
  (returns (Value :type "Float (double-precision)"))
  (bind _interactor (`self.Interactor`)
    (:`then`
      (bind _returnvalue_x (`KismetMathLibrary.BreakVector` (- (`KismetMathLibrary.InverseTransformLocation` (`self.GetTransform`) (`SceneComponent.K2_GetComponentLocation` _interactor)) (`SceneComponent.RelativeLocation` (`self.SlelfHandle`)))))
      (return _returnvalue_x))
    (:`else`)))

(fn `UserConstructionScript`)