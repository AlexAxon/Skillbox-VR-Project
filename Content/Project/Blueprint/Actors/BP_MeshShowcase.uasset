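; BP_MeshShowcase is a display actor that shows a configurable mesh with a text label and an attached commentary box.
; The construction script applies the mesh, text, size and color, then passes the commentary lines to the BP_Commentary_Box child actor.
; The label starts hidden; Lookat shows it and turns the commentary box on, while LookAway hides it and turns the box off.
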(event `self.ReceiveBeginPlay`
  (`SceneComponent.SetVisibility` (`self.TextRender`) false false))

(event `/Game/Project/Blueprint/Interfaces/BPI_LookInterface.LookAt`
  (`SceneComponent.SetVisibility` (`self.TextRender`) true false)
  (`/Game/Project/Blueprint/Interfaces/BPI_ElectricSwitchable.TurnOn` (`self.TipActorReference`)))

(event `/Game/Project/Blueprint/Interfaces/BPI_LookInterface.LookAway`
  (`SceneComponent.SetVisibility` (`self.TextRender`) false false)
  (`/Game/Project/Blueprint/Interfaces/BPI_ElectricSwitchable.TurnOff` (`self.TipActorReference`)))

(fn `UserConstructionScript`
  (`StaticMeshComponent.SetStaticMesh` (`self.StaticMesh`) (`self.Mesh`))
  (`TextRenderComponent.K2_SetText` (`self.TextRender`) (`self.Text`))
  (`TextRenderComponent.SetWorldSize` (`self.TextRender`) (`self.TextSize`))
  (`TextRenderComponent.SetTextRenderColor` (`self.TextRender`) (`self.TextColor`))
  (bind _asbp_commentary_box (cast `/Game/Assets/Blueprints/BP_Commentary_Box` (`ChildActorComponent.ChildActor` (`self.BP_Commentary_Box`))))
  (bind _output_get (set `self.TipActorReference` _asbp_commentary_box))
  (set `/Game/Assets/Blueprints/BP_Commentary_Box.Lines` (`self.Lines`) _output_get))