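; Music cube actor for a Simon-style memory game where the player repeats a random sequence of lit, sounding buttons.
; Buttons are components tagged "MusicButton"; a looping timer alternates their highlight to play the sequence, then opens input.
; Interact checks the hit component against the expected note, coloring it green or red and playing its sound.
; Completing a round rolls a new, longer sequence, while a mistake resets the progression.
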(event `self.ReceiveBeginPlay`
  (set `self.CurrentSequanceLoop` 0)
  (`self.CalculateNotes`)
  (`self.PlayNoteSequance`))

(event `/Game/Project/Blueprint/Interfaces/BPI_InteractInterface.Interact`
  (params (OutHit :type "HitResult Structure"))
  (if (`self.bIsInputMode`)
    (bind (_bsuccess _bcorrect _buttoncomponent _buttonid) (`self.TryPressButton` (`.HitComponent` (`GameplayStatics.BreakHitResult` OutHit))))
    (if _bsuccess
      (`self.InteractButton` _bcorrect _buttonid))))

(fn `CalculateNotes`
  (locals (`Local Max Notes` :type Integer :default 0))
  (`KismetArrayLibrary.Array_Clear` (`self.Notes`))
  (set `local.Local Max Notes` (`self.CurrentSequanceLoop`))
  (for _ (range (+ (`local.Local Max Notes`) 1))
    (`KismetArrayLibrary.Array_Add` (`self.Notes`) (`KismetMathLibrary.RandomInteger` (`self.ButtonsCount`))))
  (set `self.SizeOfSequance` (`KismetArrayLibrary.Array_Length` (`self.Notes`))))

(fn `ClearActiveButton`
  (bind _asstatic_mesh_component (cast `StaticMeshComponent` (`|GetArrayItem` (`self.Buttons`) (`self.ActiveButton`))))
  (`PrimitiveComponent.SetMaterial` _asstatic_mesh_component 0 "/Game/Project/Materials/M_ColorGray.M_ColorGray"))

(fn `CollectButtons`
  (`KismetArrayLibrary.Array_Clear` (`self.Buttons`))
  (set `self.Buttons` (`self.GetComponentsByTag` "/Script/Engine.ActorComponent" "MusicButton"))
  (set `self.ButtonsCount` (`KismetArrayLibrary.Array_Length` (`self.Buttons`))))

(fn `InteractButton`
  (params (Correct :type Boolean) (ButtonID :type Integer))
  (set `self.ActiveButton` ButtonID)
  (`KismetSystemLibrary.K2_SetTimer` null "ClearActiveButton" (`self.Speed`))
  (`GameplayStatics.PlaySoundAtLocation` (`|GetArrayItem` (`self.Sounds`) (`self.ActiveButton`)) (`SceneComponent.K2_GetComponentLocation` (`self.SM_MusicCube_Base`)) (struct) 1.0 1.0 0.0 null null null null))

(fn `PlayNote`
  (if (< (`self.NoteLoop`) (`self.SizeOfSequance`))
    (set `self.CurrentNote` (`|GetArrayItem` (`self.Notes`) (`self.NoteLoop`)))
    (if (`self.bIsTurnOn`)
      (set `self.bIsTurnOn` false)
      (bind _asstatic_mesh_component (cast `StaticMeshComponent` (`|GetArrayItem` (`self.Buttons`) (`self.CurrentNote`))))
      (`PrimitiveComponent.SetMaterial` _asstatic_mesh_component 0 "/Game/Project/Materials/M_ColorGreen.M_ColorGreen")
      (`GameplayStatics.PlaySoundAtLocation` (`|GetArrayItem` (`self.Sounds`) (`self.CurrentNote`)) (`SceneComponent.K2_GetComponentLocation` (`self.SM_MusicCube_Base`)) (struct) 1.0 1.0 0.0 null null null null)
      (else
        (set `self.bIsTurnOn` true)
        (bind _asstatic_mesh_component_2 (cast `StaticMeshComponent` (`|GetArrayItem` (`self.Buttons`) (`self.CurrentNote`))))
        (`PrimitiveComponent.SetMaterial` _asstatic_mesh_component_2 0 "/Game/Project/Materials/M_ColorGray.M_ColorGray")
        (`/Engine/EditorBlueprintResources/StandardMacros.IncrementInt` (`self.NoteLoop`))))
    (else
      (`KismetSystemLibrary.K2_ClearAndInvalidateTimerHandle` (`self.Play Note Timer Handle`))
      (set `self.bIsInputMode` true)
      (set `self.NoteLoop` 0))))

(fn `PlayNoteSequance`
  (set `self.bIsInputMode` false)
  (set `self.NoteLoop` 0)
  (bind _returnvalue (`KismetSystemLibrary.K2_SetTimer` null "PlayNote" (`self.Speed`) true))
  (set `self.Play Note Timer Handle` _returnvalue)
  (`TextRenderComponent.K2_SetText` (`self.TextRender`) (`KismetTextLibrary.Conv_IntToText` (`self.SizeOfSequance`))))

(fn `TryPressButton`
  (params (Object :type "ActorComponent Object Reference"))
  (returns (bSuccess :type Boolean) (bCorrect :type Boolean) (ButtonComponent :type "StaticMeshComponent Object Reference") (ButtonID :type Integer))
  (locals (LocalButton :type "StaticMeshComponent Object Reference") (LocalButtonID :type Integer :default 0))
  (bind _asstatic_mesh_component (cast `StaticMeshComponent` Object)
    (:`then`
      (bind _output_get (set `local.LocalButton` _asstatic_mesh_component))
      (bind _returnvalue (`KismetArrayLibrary.Array_Find` (`self.Buttons`) _output_get))
      (set `local.LocalButtonID` _returnvalue)
      (if (== _returnvalue (`|GetArrayItem` (`self.Notes`) (`self.NoteLoop`)))
        (`PrimitiveComponent.SetMaterial` (`local.LocalButton`) 0 "/Game/Project/Materials/M_ColorGreen.M_ColorGreen")
        (`/Engine/EditorBlueprintResources/StandardMacros.IncrementInt` (`self.NoteLoop`)
          (:`  `
            (if (>= (`self.NoteLoop`) (`self.SizeOfSequance`))
              (`self.UpdateGameLoop`))
            (return true true (`local.LocalButton`) (`local.LocalButtonID`))))
        (else
          (`PrimitiveComponent.SetMaterial` (`local.LocalButton`) 0 "/Game/Project/Materials/M_ColorRed.M_ColorRed")
          (set `self.CurrentSequanceLoop` 0)
          (`self.UpdateGameLoop`)
          (return true false (`local.LocalButton`) (`local.LocalButtonID`)))))
    (:`CastFailed`
      (return false false null 0))))

(fn `UpdateBaseColors`
  (`PrimitiveComponent.SetMaterial` (`self.SM_MusicCube_Base`) 0 "/Game/Project/Materials/M_ColorBlue.M_ColorBlue"))

(fn `UpdateGameLoop`
  (`/Engine/EditorBlueprintResources/StandardMacros.IncrementInt` (`self.CurrentSequanceLoop`)
    (:`  `
      (`self.CalculateNotes`)
      (`self.PlayNoteSequance`))))

(fn `UserConstructionScript`
  (`self.UpdateBaseColors`)
  (`self.CollectButtons`))