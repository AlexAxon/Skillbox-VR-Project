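; BP_TraceObject is a display object with a configurable mesh and text label that can spin and show or hide its info.
; The construction script applies the Mesh and Text variables to the StaticMesh and TextRender components.
; Activate and Deactivate open and close a Gate on Tick that adds a fixed local rotation each frame, so spin speed depends on frame rate.
; ToggleInfo flips the text's visibility.
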(event `self.ReceiveTick`
  (params (DeltaSeconds :type "Float (single-precision)"))
  (`/Engine/EditorBlueprintResources/StandardMacros.Gate` true :!label _label
    (:`Exit`
      (`SceneComponent.K2_AddLocalRotation` (`self.StaticMesh`) (struct :`Yaw` 1.0) false false))))

(event `Activate`
  (goto _label :!via `Open`))

(event `Deactivate`
  (goto _label :!via `Close`))

(event `ToggleInfo`
  (`SceneComponent.SetVisibility` (`self.TextRender`) (not (`SceneComponent.bVisible` (`self.TextRender`))) false))

(fn `UserConstructionScript`
  (`StaticMeshComponent.SetStaticMesh` (`self.StaticMesh`) (`self.Mesh`))
  (`TextRenderComponent.K2_SetText` (`self.TextRender`) (`self.Text`)))